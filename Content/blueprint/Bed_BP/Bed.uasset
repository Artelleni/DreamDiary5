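; Bed actor that lets the player start dreaming after a countdown triggered by colliding with it.
; A hit on its Box component by PlayerBP sets a collision flag that is never cleared, so Tick decrements Delay every frame thereafter and prints it.
; On a later hit, if the player has hit Enter and Delay has run out, it sets PlayerCanDream on PlayerBP.
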(event `self.ReceiveTick`
  (params (DeltaSeconds :type "Float (single-precision)"))
  (if (`self.PlayerColided`)
    (bind _result (`/Engine/EditorBlueprintResources/StandardMacros.DecrementFloat` (`self.Delay`))
      (:`  `
        (`KismetSystemLibrary.PrintString` (`KismetStringLibrary.Conv_DoubleToString` _result))))))

(event `self.Box.OnComponentHit`
  (params (HitComponent :type "PrimitiveComponent Object Reference") (OtherActor :type "Actor Object Reference") (OtherComp :type "PrimitiveComponent Object Reference") (NormalImpulse :type "Vector Structure") (Hit :type "HitResult Structure (by ref)"))
  (bind _asplayer_bp (cast `/Game/blueprint/Player_BP/PlayerBP` OtherActor))
  (set `self.PlayerColided` true)
  (if (`/Game/blueprint/Player_BP/PlayerBP.PlayerHasHitEnter` _asplayer_bp)
    (if (<= (`self.Delay`) 0.0)
      (set `/Game/blueprint/Player_BP/PlayerBP.PlayerCanDream` true _asplayer_bp))))

(fn `UserConstructionScript`)