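; Player pawn Blueprint that handles planar movement and a screen-size toggle.
; MoveLeft and MoveUp axes drive movement input along the forward and right vectors respectively, using only control rotation yaw to stay on the plane.
; FullScreen_Action flips IsFullScreen and applies a 320x240 or 640x480 resolution through GameUserSettings, changing resolution only, not window mode.
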(event `InputAction|FullScreen_Action`
  (params (Key :type "Key Structure"))
  ;[1 1 1] Change Screen Size
  (:`Pressed`
    (if (`self.IsFullScreen`)
      (bind _returnvalue (`GameUserSettings.GetGameUserSettings`))
      (`GameUserSettings.SetScreenResolution` _returnvalue (make `IntPoint` 320 240))
      (`GameUserSettings.ApplySettings` _returnvalue true)
      (set `self.IsFullScreen` false)
      (else
        (bind _returnvalue_2 (`GameUserSettings.GetGameUserSettings`))
        (`GameUserSettings.SetScreenResolution` _returnvalue_2 (make `IntPoint` 640 480))
        (`GameUserSettings.ApplySettings` _returnvalue_2 true)
        (set `self.IsFullScreen` true)))))

(event `InputAxis|MoveLeft`
  (params (AxisValue :type "Float (single-precision)"))
  ;[1 1 1] Player Movement
  (`self.AddMovementInput` (`KismetMathLibrary.GetForwardVector` (`KismetMathLibrary.MakeRotator` 0.0 0.0 (.yaw (`self.GetControlRotation`)))) AxisValue))

(event `InputAxis|MoveUp`
  (params (AxisValue :type "Float (single-precision)"))
  ;[1 1 1] Player Movement
  (`self.AddMovementInput` (`KismetMathLibrary.GetRightVector` (`KismetMathLibrary.MakeRotator` 0.0 0.0 (.yaw (`self.GetControlRotation`)))) AxisValue))

(fn `UserConstructionScript`)