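; Player character Blueprint that moves along the world X axis and switches between walking and flying.
; Axis inputs add movement and set direction flags, though MoveUp passes a zero direction vector.
; Every Tick, CheckIfUp reads the up and down flags, calling EnableFlying when either is set and restoring Walking otherwise.
; EnableFlying sets Flying mode while also raising gravity scale and enabling gravity on capsule and Player component.
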(event `self.ReceiveTick`
  (params (DeltaSeconds :type "Float (single-precision)"))
  (`self.CheckIfUp` (`self.MovingUp`) (`self.MovingDown`)))

(event `InputAxis|MoveLeft`
  (params (AxisValue :type "Float (single-precision)"))
  (if (> AxisValue 0.0)
    (set `self.bisMovingRight` true)
    (`self.AddMovementInput` (1.0 0.0 0.0) AxisValue :!label _label)
    (elif (< AxisValue 0.0)
      (set `self.bisMovingRight` false)
      (goto _label))))

(event `InputAxis|MoveUp`
  (params (AxisValue :type "Float (single-precision)"))
  (if (> AxisValue 0.0)
    (set `self.MovingUp` true)
    (`self.AddMovementInput` (0.0 0.0 0.0) AxisValue :!label _label_2)
    (else
      (set `self.MovingUp` false)
      (if (< AxisValue 0.0)
        (set `self.MovingDown` true)
        (goto _label_2)
        (else
          (set `self.MovingDown` false))))))

(fn `CheckIfUp`
  (params (NewParam :type Boolean) (NewParam1 :type Boolean))
  (if NewParam
    (`self.EnableFlying` :!label _label)
    (elif NewParam1
      (goto _label)
      (else
        (`CharacterMovementComponent.SetMovementMode` (`self.CharacterMovement`) "MOVE_Walking" 0)))))

(fn `EnableFlying`
  (set `CharacterMovementComponent.GravityScale` 2.0 (`self.CharacterMovement`))
  (`PrimitiveComponent.SetEnableGravity` (`self.CapsuleComponent`) true)
  (`PrimitiveComponent.SetEnableGravity` (`self.Player`) true)
  (`CharacterMovementComponent.SetMovementMode` (`self.CharacterMovement`) "MOVE_Flying" 0))

(fn `UserConstructionScript`)