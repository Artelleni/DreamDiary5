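; Scooter pickup actor that switches the player to scooter idle and walk animations, sets walk speed and destroys itself.
; An EffectZone overlap with PlayerBP sets a flag, which Tick polls to apply the effect through the Player variable.
; Pickup flags the first loadable of three save slots, though the third saves into the second's name.
; BeginPlay async-saves a fresh save object, then async-loads it, destroying the actor if already equipped.
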(event `self.ReceiveBeginPlay`
  (bind _savegame (`self.SaveGame`))
  (`|ExecutionSequence`
    (:`then_0`
      (bind _returnvalue (`GameplayStatics.CreateSaveGameObject` "/Game/SaveSlot/SaveGameSlot.SaveGameSlot_C"))
      (bind _output_get (set `self.SaveGame` _returnvalue))
      (bind (_savegame_2 _bsuccess) (`AsyncActionHandleSaveGame.AsyncSaveGameToSlot` _output_get (`/Game/SaveSlot/SaveGameSlot.SaveSlot` _output_get) (`/Game/SaveSlot/SaveGameSlot.userindex` _output_get))
        (:`Completed`
          (`KismetSystemLibrary.PrintString` (`KismetStringLibrary.Conv_BoolToString` _bsuccess)))))
    (:`then_1`
      (bind (_savegame_3 _bsuccess_2) (`AsyncActionHandleSaveGame.AsyncLoadGameFromSlot` (`/Game/SaveSlot/SaveGameSlot.SaveSlot` _savegame) (`/Game/SaveSlot/SaveGameSlot.userindex` _savegame))
        (:`Completed`
          (bind _assave_game_slot (cast `/Game/SaveSlot/SaveGameSlot` _savegame_3)
            (:`then`
              (if (`/Game/SaveSlot/SaveGameSlot.PlayerHasEquippedScooter` _assave_game_slot)
                (`self.K2_DestroyActor`)
                (else
                  (`KismetSystemLibrary.PrintString` "has not picked up"))))
            (:`CastFailed`
              (`KismetSystemLibrary.PrintString` (`KismetStringLibrary.Conv_BoolToString` _bsuccess_2) true true (struct :`R` 1.0 :`G` 0.109946 :`A` 1.0)))))))))

(event `self.ReceiveTick`
  (params (DeltaSeconds :type "Float (single-precision)"))
  (`self.OnColllsionWithPlayerEquip` (`self.HasColided`) (`self.Player`)))

(event `self.EffectZone.OnComponentBeginOverlap`
  (params (OverlappedComponent :type "PrimitiveComponent Object Reference") (OtherActor :type "Actor Object Reference") (OtherComp :type "PrimitiveComponent Object Reference") (OtherBodyIndex :type Integer) (bFromSweep :type Boolean) (SweepResult :type "HitResult Structure (by ref)"))
  (cast `/Game/blueprint/Player_BP/PlayerBP` OtherActor)
  (set `self.HasColided` true))

(fn `OnColllsionWithPlayerEquip`
  (params (NewParam :type Boolean) (Player :type "/Game/blueprint/Player_BP/PlayerBP Object Reference"))
  (if NewParam
    (`|ExecutionSequence`
      (:`then_0`
        (set `/Game/blueprint/Player_BP/PlayerBP.Idle` (`self.PlayerScooterIdle`) Player))
      (:`then_1`
        (set `/Game/blueprint/Player_BP/PlayerBP.WalkDown` (`self.PlauerScooterDown`) Player))
      (:`then_2`
        (set `/Game/blueprint/Player_BP/PlayerBP.WalkLeft` (`self.PlayerScooterLeft`) Player))
      (:`then_3`
        (set `/Game/blueprint/Player_BP/PlayerBP.WalkRight` (`self.PlayerScotterRight`) Player))
      (:`then_4`
        (set `/Game/blueprint/Player_BP/PlayerBP.WalkUp` (`self.PlayerScooterUp`) Player))
      (:`then_5`
        (set `CharacterMovementComponent.MaxWalkSpeed` 150.0 (`Character.CharacterMovement` Player)))
      (:`then_6`
        (bind _returnvalue (`GameplayStatics.LoadGameFromSlot` "SaveSlot0"))
        (bind _assave_game_slot (cast `/Game/SaveSlot/SaveGameSlot` _returnvalue)
          (:`then`
            (set `/Game/SaveSlot/SaveGameSlot.PlayerHasEquippedScooter` true _assave_game_slot)
            (`GameplayStatics.SaveGameToSlot` _assave_game_slot "SaveSlot0"))
          (:`CastFailed`
            (bind _returnvalue_2 (`GameplayStatics.LoadGameFromSlot` "SaveSlot1"))
            (bind _assave_game_slot_2 (cast `/Game/SaveSlot/SaveGameSlot` _returnvalue_2)
              (:`then`
                (set `/Game/SaveSlot/SaveGameSlot.PlayerHasEquippedScooter` true _assave_game_slot_2)
                (`GameplayStatics.SaveGameToSlot` _assave_game_slot_2 "SaveSlot1"))
              (:`CastFailed`
                (bind _returnvalue_3 (`GameplayStatics.LoadGameFromSlot` "SaveSlot2"))
                (bind _assave_game_slot_3 (cast `/Game/SaveSlot/SaveGameSlot` _returnvalue_3))
                (set `/Game/SaveSlot/SaveGameSlot.PlayerHasEquippedScooter` true _assave_game_slot_3)
                (`GameplayStatics.SaveGameToSlot` _assave_game_slot_3 "SaveSlot1"))))))
      (:`then_7`
        (`self.K2_DestroyActor`)))))

(fn `UserConstructionScript`)